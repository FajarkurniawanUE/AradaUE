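; Interaction actor for an elevator that highlights the elevator mesh and accepts the Interact input while the player is looking at it.
; BeginPlay caches the player character and controller, and Tick compares the controller's current traced actor to the elevator mesh actor.
; Paired DoOnce nodes toggle custom depth on changes, while input is enabled or disabled to match.
; Interact only prints a placeholder for opening the elevator menu.
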(event Custom|beingTrace
  (Input|EnableInput (Game|GetPlayerController 0))
  (Utilities|FlowControl|Sequence
    (:then_0
      (Utilities|FlowControl|DoOnce false
        (:Completed
          (Rendering|SetRenderCustomDepth (Variables|/Script/Engine.StaticMeshActor|GetStaticMeshComponent (Variables|Default|GetElevator%20SM)) true))))
    (:then_1
      (Utilities|FlowControl|DoOnce false) ; enters at Reset
    )))

(event Custom|notTrace
  (Input|DisableInput (Game|GetPlayerController 0))
  (Utilities|FlowControl|Sequence
    (:then_0
      (Utilities|FlowControl|DoOnce false) ; enters at Reset
    )
    (:then_1
      (Utilities|FlowControl|DoOnce false
        (:Completed
          (Rendering|SetRenderCustomDepth (Variables|/Script/Engine.StaticMeshActor|GetStaticMeshComponent (Variables|Default|GetElevator%20SM)) false))))))

(event EventBeginPlay
  (Utilities|FlowControl|Sequence
    (:then_0
      (bind _aschar_arada_walk (Utilities|Casting|CastTochar_arada_walk (Game|GetPlayerCharacter 0)))
      (Variables|Default|SetAs%20Char%20Arada%20Walk _aschar_arada_walk))
    (:then_1
      (bind _aspc_arada (Utilities|Casting|CastTopc_arada (Game|GetPlayerController 0)))
      (Variables|Default|SetAs%20Pc%20Arada _aspc_arada))))

(event EventTick
  (params (DeltaSeconds :type Float%20%28single-precision%29))
  (if (== (Variables|/Game/Arada_Fajar/Blueprints/pc_arada.pc_arada_C|GetCurrentTracingActor (Variables|Default|GetAs%20Pc%20Arada)) (Variables|Default|GetElevator%20SM))
    (CallFunction|BeingTrace)
    (else
      (CallFunction|NotTrace))))

(event Input|ActionEvents|InputActionInteract
  (params (Key :type Key%20Structure :default "None"))
  (:Pressed
    (Development|PrintString "OPEN ELEVATOR MENU")))

(fn ConstructionScript)